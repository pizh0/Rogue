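; Oppressor is an automatic shotgun weapon that fires bursts of pellets and reloads from the player character's shotgun ammo reserve.
; While the fire flag is set, FireStarts loops on a delay, spending one round per SpawnDrob call, which spawns randomly spread ShotBul3 projectiles from Boom.
; Reload logic, duplicated in an event and StartReload, tops up the magazine from ShotAmmoInv.
; Empty firing and full-magazine reloads play a sound.
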(event Custom|FireStarts
  (if (Variables|Default|GetFire) :!label _label
    (if (> (Variables|Default|GetAmmoCur) 0)
      (Variables|Default|SetKD true)
      (CallFunction|SpawnDrob)
      (Audio|PlaySound2D "/Game/Sounds/Weapon/WingmanShot.WingmanShot" 1.0 1.0 0.0 0 0)
      (bind _result (Math|Integer|DecrementInt (Variables|Default|GetAmmoCur))
        (:%20%20
          (Development|PrintString (Utilities|String|ToString(Integer) _result))
          (Utilities|FlowControl|Delay 0.5)
          (goto _label)))
      (else
        (Audio|PlaySound2D "/Game/Sounds/Char/anime-moan-meme.anime-moan-meme" 1.0 1.0 0.0 0 0)))))

(event Custom|Start
  (params (NumberOfSlot :type Integer)))

(event Custom|Reload
  (bind _as_char_bp (Variables|Default|GetAs%20Char%20BP))
  (if (< (Variables|Default|GetAmmoCur) (Variables|Default|GetAmmoMax))
    (if (>= (Variables|/Game/Char/Char_BP.Char_BP_C|GetShotAmmoInv (Variables|Default|GetAs%20Char%20BP)) (- (Variables|Default|GetAmmoMax) (Variables|Default|GetAmmoCur)))
      (Variables|/Game/Char/Char_BP.Char_BP_C|SetShotAmmoInv _as_char_bp (- (Variables|/Game/Char/Char_BP.Char_BP_C|GetShotAmmoInv _as_char_bp) (- (Variables|Default|GetAmmoMax) (Variables|Default|GetAmmoCur))))
      (bind _output_get (Variables|Default|SetAmmoCur (+ (Variables|Default|GetAmmoCur) (- (Variables|Default|GetAmmoMax) (Variables|Default|GetAmmoCur)))))
      (Development|PrintString (Utilities|String|ToString(Integer) _output_get))
      (else
        (bind _output_get_2 (Variables|Default|SetAmmoCur (+ (Variables|Default|GetAmmoCur) (Variables|/Game/Char/Char_BP.Char_BP_C|GetShotAmmoInv (Variables|Default|GetAs%20Char%20BP)))))
        (Variables|/Game/Char/Char_BP.Char_BP_C|SetShotAmmoInv (Variables|Default|GetAs%20Char%20BP) 0)
        (Development|PrintString (Utilities|String|ToString(Integer) _output_get_2))))
    (else
      (Audio|PlaySound2D "/Game/Sounds/Char/anime-moan-meme.anime-moan-meme" 1.0 1.0 0.0 0 0))))

(event EventBeginPlay
  (Variables|Default|SetAmmoCur (Variables|Default|GetAmmoMax))
  (bind _aschar_bp (Utilities|Casting|CastToChar_BP (Game|Player|GetPlayerPawn 0)))
  (Variables|Default|SetAs%20Char%20BP _aschar_bp))

(event Collision|EventActorBeginOverlap
  (params (OtherActor :type Actor%20Object%20Reference)))

(event EventTick
  (params (DeltaSeconds :type Float%20%28single-precision%29)))

(fn ConstructionScript)

(fn SpawnDrob
  (bind _self self)
  (bind _boom (Variables|Default|GetBoom))
  (bind _returnvalue (Transformation|GetWorldTransform _boom))
  (for _index (range 1 10)
    (Game|SpawnActorfromClass "/Game/Weapon/Oppressor/ShotBul3.ShotBul3_C" (Math|Transform|MakeTransform (.location _returnvalue) (Math|Rotator|MakeRotator (+ (.roll (.rotation _returnvalue)) (Math|Random|RandomFloatinRange -5.0 5.0)) (+ (.pitch (.rotation _returnvalue)) (Math|Random|RandomFloatinRange -5.0 5.0)) (+ (.yaw (.rotation _returnvalue)) (Math|Random|RandomFloatinRange -5.0 5.0))) "1,1,1") "AlwaysSpawn" _self _self))
  (return false))

(fn GetAmmo
  (return (Variables|Default|GetAmmoCur)))

(fn StartFire
  (Variables|Default|SetFire true)
  (CallFunction|FireStarts)
  (return false))

(fn StartReload
  (bind _as_char_bp (Variables|Default|GetAs%20Char%20BP))
  (if (< (Variables|Default|GetAmmoCur) (Variables|Default|GetAmmoMax))
    (if (>= (Variables|/Game/Char/Char_BP.Char_BP_C|GetShotAmmoInv (Variables|Default|GetAs%20Char%20BP)) (- (Variables|Default|GetAmmoMax) (Variables|Default|GetAmmoCur)))
      (Variables|/Game/Char/Char_BP.Char_BP_C|SetShotAmmoInv _as_char_bp (- (Variables|/Game/Char/Char_BP.Char_BP_C|GetShotAmmoInv _as_char_bp) (- (Variables|Default|GetAmmoMax) (Variables|Default|GetAmmoCur))))
      (bind _output_get (Variables|Default|SetAmmoCur (+ (Variables|Default|GetAmmoCur) (- (Variables|Default|GetAmmoMax) (Variables|Default|GetAmmoCur)))))
      (Development|PrintString (Utilities|String|ToString(Integer) _output_get))
      (else
        (bind _output_get_2 (Variables|Default|SetAmmoCur (+ (Variables|Default|GetAmmoCur) (Variables|/Game/Char/Char_BP.Char_BP_C|GetShotAmmoInv (Variables|Default|GetAs%20Char%20BP)))))
        (Variables|/Game/Char/Char_BP.Char_BP_C|SetShotAmmoInv (Variables|Default|GetAs%20Char%20BP) 0)
        (Development|PrintString (Utilities|String|ToString(Integer) _output_get_2))))
    (return false)
    (else
      (Audio|PlaySound2D "/Game/Sounds/Char/anime-moan-meme.anime-moan-meme" 1.0 1.0 0.0 0 0))))

(fn StopFire
  (Variables|Default|SetFire false)
  (return false))