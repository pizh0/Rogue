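; PP_BP is an automatic weapon that fires Bullet actors from its Boom component and tracks its own ammo.
; StartFire starts a 0.1-second Delay loop that spawns bullets with sound until StopFire clears the flag or ammo runs out.
; Bullets fired while the player character is falling get a Boomnah call.
; StartReload refills the magazine from the character's LightAmmoInv, taking whatever remains when short.
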(event Custom|FireStarts
  (bind _self self)
  (bind _boom (Variables|Default|GetBoom))
  (bind _returnvalue (Transformation|GetWorldTransform _boom))
  (if (Variables|Default|GetFire) :!label _label
    (if (> (Variables|Default|GetAmmoCur) 0)
      (bind _returnvalue_2 (Game|SpawnActorfromClass "/Game/Weapon/Common/Bullet.Bullet_C" (Math|Transform|MakeTransform (.location _returnvalue) (.rotation _returnvalue) "1,1,1") "Undefined" _self _self))
      (if (AI|Components|NavMovement|IsFalling (Pawn|GetMovementComponent (Variables|Default|GetAs%20Char%20BP)))
        (Default|Boomnah _returnvalue_2))
      (Audio|PlaySound2D "/Game/Sounds/Char/pew-pew-lame-sound-effect.pew-pew-lame-sound-effect" 1.0 1.0 0.0 0 0)
      (bind _result (Math|Integer|DecrementInt (Variables|Default|GetAmmoCur))
        (:%20%20
          (Development|PrintString (Utilities|String|ToString(Integer) _result))
          (Utilities|FlowControl|Delay 0.1)
          (goto _label)))
      (else
        (Audio|PlaySound2D "/Game/Sounds/Char/anime-moan-meme.anime-moan-meme" 1.0 1.0 0.0 0 0)))))

(event EventBeginPlay
  (Variables|Default|SetAmmoCur (Variables|Default|GetAmmoMax))
  (bind _aschar_bp (Utilities|Casting|CastToChar_BP (Game|Player|GetPlayerPawn 0)))
  (Variables|Default|SetAs%20Char%20BP _aschar_bp))

(event Collision|EventActorBeginOverlap
  (params (OtherActor :type Actor%20Object%20Reference)))

(event EventTick
  (params (DeltaSeconds :type Float%20%28single-precision%29)))

(fn ConstructionScript)

(fn GetAmmo
  (return (Variables|Default|GetAmmoCur)))

(fn StartFire
  (Variables|Default|SetFire true)
  (CallFunction|FireStarts)
  (return false))

(fn StartReload
  (bind _as_char_bp (Variables|Default|GetAs%20Char%20BP))
  (if (< (Variables|Default|GetAmmoCur) (Variables|Default|GetAmmoMax))
    (if (>= (Variables|/Game/Char/Char_BP.Char_BP_C|GetLightAmmoInv (Variables|Default|GetAs%20Char%20BP)) (- (Variables|Default|GetAmmoMax) (Variables|Default|GetAmmoCur)))
      (Development|PrintString "Hello")
      (Variables|/Game/Char/Char_BP.Char_BP_C|SetLightAmmoInv _as_char_bp (- (Variables|/Game/Char/Char_BP.Char_BP_C|GetLightAmmoInv _as_char_bp) (- (Variables|Default|GetAmmoMax) (Variables|Default|GetAmmoCur))))
      (Variables|Default|SetAmmoCur (+ (Variables|Default|GetAmmoCur) (- (Variables|Default|GetAmmoMax) (Variables|Default|GetAmmoCur))))
      (else
        (Development|PrintString "нет")
        (Variables|Default|SetAmmoCur (+ (Variables|Default|GetAmmoCur) (Variables|/Game/Char/Char_BP.Char_BP_C|GetLightAmmoInv (Variables|Default|GetAs%20Char%20BP))))
        (Variables|/Game/Char/Char_BP.Char_BP_C|SetLightAmmoInv (Variables|Default|GetAs%20Char%20BP) 0)))
    (return false)
    (else
      (Audio|PlaySound2D "/Game/Sounds/Char/anime-moan-meme.anime-moan-meme" 1.0 1.0 0.0 0 0))))

(fn StopFire
  (Variables|Default|SetFire false)
  (return false))