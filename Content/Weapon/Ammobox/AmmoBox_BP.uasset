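; AmmoBox_BP is a pickup that gives the player both ammo and healing.
; On Box overlap by the player pawn, it calls PickUpAmmo on Char_BP and destroys itself, but only if the character's ammo inventory or HP is below maximum.
; The root component's world X scale, read at BeginPlay, multiplies the default ammo and heal amounts, so a box's size sets its value.
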(event OnComponentBeginOverlap(Box)
  (params (OverlappedComponent :type Primitive%20Component%20Object%20Reference) (OtherActor :type Actor%20Object%20Reference) (OtherComp :type Primitive%20Component%20Object%20Reference) (OtherBodyIndex :type Integer) (bFromSweep :type Boolean) (SweepResult :type Hit%20Result%20Structure%20%28by%20ref%29))
  (bind _q (Variables|Default|GetQ))
  (if (== OtherActor (Game|Player|GetPlayerPawn 0))
    (bind _aschar_bp (Utilities|Casting|CastToChar_BP OtherActor))
    (if (not (Math|Boolean|NORBoolean (< (Variables|/Game/Char/Char_BP.Char_BP_C|GetAmmoInv _aschar_bp) (Variables|/Game/Char/Char_BP.Char_BP_C|GetMaxAmmoInv _aschar_bp)) (< (Variables|/Game/Char/Char_BP.Char_BP_C|GetHP _aschar_bp) (Variables|/Game/Char/Char_BP.Char_BP_C|GetMaxHP _aschar_bp))))
      (Default|PickUpAmmo _aschar_bp (Math|Float|Truncate (* (Variables|Default|GetDefaultAmmo) _q)) (* (Variables|Default|GetDefailtHeal) _q))
      (Actor|DestroyActor))))

(event EventBeginPlay
  (Variables|Default|SetQ (.x (Transformation|GetWorldScale (Variables|Default|GetDefaultSceneRoot)))))

(event Collision|EventActorBeginOverlap
  (params (OtherActor :type Actor%20Object%20Reference)))

(event EventTick
  (params (DeltaSeconds :type Float%20%28single-precision%29)))

(fn ConstructionScript)