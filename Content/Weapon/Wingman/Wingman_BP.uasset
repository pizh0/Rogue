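; Wingman weapon Blueprint that fires projectiles and manages its magazine using the player's heavy ammo inventory.
; While Fire is set, a delayed loop spawns WingmanBullet at the Boom transform, plays a shot sound and decrements ammo, playing another sound when empty.
; StartFire and StopFire toggle that flag.
; StartReload refills from the player character's HeavyAmmoInv, taking whatever remains if short.
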(event Custom|FireStarts
  (bind _self self)
  (bind _boom (Variables|Default|GetBoom))
  (bind _returnvalue (Transformation|GetWorldTransform _boom))
  (if (Variables|Default|GetFire) :!label _label
    (if (> (Variables|Default|GetAmmoCur) 0)
      (Game|SpawnActorfromClass "/Game/Weapon/Wingman/WingmanBullet.WingmanBullet_C" (Math|Transform|MakeTransform (.location _returnvalue) (.rotation _returnvalue) "1,1,1") "Undefined" _self 5e+04 true true true "NewEnumerator2" 0 "NewEnumerator0" _self)
      (Audio|PlaySound2D "/Game/Sounds/Weapon/WingmanShot.WingmanShot" 1.0 1.0 0.0 0 0)
      (bind _result (Math|Integer|DecrementInt (Variables|Default|GetAmmoCur))
        (:%20%20
          (Development|PrintString (Utilities|String|ToString(Integer) _result))
          (Utilities|FlowControl|Delay 0.5)
          (goto _label)))
      (else
        (Audio|PlaySound2D "/Game/Sounds/Char/anime-moan-meme.anime-moan-meme" 1.0 1.0 0.0 0 0)))))

(event EventBeginPlay
  (Variables|Default|SetAmmoCur (Variables|Default|GetAmmoMax))
  (bind _aschar_bp (Utilities|Casting|CastToChar_BP (Game|Player|GetPlayerPawn 0)))
  (Variables|Default|SetAs%20Char%20BP _aschar_bp))

(event Collision|EventActorBeginOverlap
  (params (OtherActor :type Actor%20Object%20Reference)))

(event EventTick
  (params (DeltaSeconds :type Float%20%28single-precision%29)))

(fn ConstructionScript)

(fn GetAmmo
  (return (Variables|Default|GetAmmoCur)))

(fn StartFire
  (Variables|Default|SetFire true)
  (CallFunction|FireStarts)
  (return false))

(fn StartReload
  (bind _as_char_bp (Variables|Default|GetAs%20Char%20BP))
  (if (< (Variables|Default|GetAmmoCur) (Variables|Default|GetAmmoMax))
    (if (>= (Variables|/Game/Char/Char_BP.Char_BP_C|GetHeavyAmmoInv (Variables|Default|GetAs%20Char%20BP)) (- (Variables|Default|GetAmmoMax) (Variables|Default|GetAmmoCur)))
      (Development|PrintString "Hello")
      (Variables|/Game/Char/Char_BP.Char_BP_C|SetHeavyAmmoInv _as_char_bp (- (Variables|/Game/Char/Char_BP.Char_BP_C|GetHeavyAmmoInv _as_char_bp) (- (Variables|Default|GetAmmoMax) (Variables|Default|GetAmmoCur))))
      (Variables|Default|SetAmmoCur (+ (Variables|Default|GetAmmoCur) (- (Variables|Default|GetAmmoMax) (Variables|Default|GetAmmoCur))))
      (return false)
      (else
        (Development|PrintString "нет")
        (Variables|Default|SetAmmoCur (+ (Variables|Default|GetAmmoCur) (Variables|/Game/Char/Char_BP.Char_BP_C|GetHeavyAmmoInv (Variables|Default|GetAs%20Char%20BP))))
        (Variables|/Game/Char/Char_BP.Char_BP_C|SetHeavyAmmoInv (Variables|Default|GetAs%20Char%20BP) 0)))
    (else
      (Audio|PlaySound2D "/Game/Sounds/Char/anime-moan-meme.anime-moan-meme" 1.0 1.0 0.0 0 0))))

(fn StopFire
  (Variables|Default|SetFire false)
  (return false))