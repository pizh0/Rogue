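; WingmanBullet_BP is the bullet actor for the Wingman weapon, dealing damage on impact.
; Its Sphere1 collision ignores the player pawn while moving and, on hit, prints the target's name, applies damage, spawns an explosion and destroys the bullet.
; The boomnah event flags a boosted shot with tenfold damage and a larger explosion.
; The hit filter ANDs its player, self and owner checks, so it excludes practically nothing.
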(event OnComponentHit(Sphere1)
  (params (HitComponent :type Primitive%20Component%20Object%20Reference) (OtherActor :type Actor%20Object%20Reference) (OtherComp :type Primitive%20Component%20Object%20Reference) (NormalImpulse :type Vector :default "0, 0, 0") (Hit :type Hit%20Result%20Structure%20%28by%20ref%29))
  (bind _basedamage (Variables|Default|GetBaseDamage))
  (if (not (and (and (== OtherActor (Game|Player|GetPlayerPawn 0)) (== OtherActor self)) (== OtherActor (Components|GetOwner))))
    (Development|PrintString (Utilities|GetDisplayName OtherActor))
    (if (Variables|Default|GetBoomNahh)
      (Variables|Default|SetDamage (* _basedamage 1e+01))
      (else
        (Variables|Default|SetDamage _basedamage)))
    (Game|Damage|ApplyDamage OtherActor (Variables|Default|GetDamage) 0 0)
    (if (Variables|Default|GetBoomNahh)
      (Effects|SpawnEmitteratLocation "/Game/StarterContent/Particles/P_Explosion.P_Explosion" (.location Hit) "0, 0, 0" "0.100000,0.100000,0.100000")
      (else
        (Effects|SpawnEmitteratLocation "/Game/StarterContent/Particles/P_Explosion.P_Explosion" (.location Hit) "0, 0, 0" "0.050000,0.050000,0.050000")))
    (Actor|DestroyActor)))

(event Custom|boomnah
  (Variables|Default|SetBoomNahh true))

(event EventBeginPlay
  (Collision|IgnoreActorwhenMoving (Variables|Default|GetSphere1) (Game|Player|GetPlayerPawn 0) true))

(fn ConstructionScript)