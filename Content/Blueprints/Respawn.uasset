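; Respawn Blueprint that spawns AI pawns at random TargetPoint actors in the level.
; The Respawn event stores the given Pawn and behavior Tree, gathers all TargetPoints, then spawns a new AI of that pawn's class running that tree.
; Location and rotation use separate random picks, so they can come from different points.
; The Bruh event repeats the spawn using the stored values and the point list gathered by Respawn.
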(event Custom|Respawn
  (params (Pawn :type Pawn%20Object%20Reference) (Tree :type Behavior%20Tree%20Object%20Reference))
  (Variables|Default|SetPawn Pawn)
  (Variables|Default|SetTree Tree)
  (bind _outactors (Actor|GetAllActorsOfClass "/Script/Engine.TargetPoint"))
  (AI|SpawnAIFromClass (Utilities|GetClass Pawn) Tree (Transformation|GetActorLocation (Utilities|Array|Get(acopy) _outactors (Math|Random|RandomIntegerinRange 0 (Utilities|Array|LastIndex _outactors)))) (Transformation|GetActorRotation (Utilities|Array|Get(acopy) _outactors (Math|Random|RandomIntegerinRange 0 (Utilities|Array|LastIndex _outactors)))) false 0))

(event Custom|Bruh
  (AI|SpawnAIFromClass (Utilities|GetClass (Variables|Default|GetPawn)) (Variables|Default|GetTree) (Transformation|GetActorLocation (Utilities|Array|Get(acopy) (stale Custom|Respawn _outactors) (Math|Random|RandomIntegerinRange 0 (Utilities|Array|LastIndex (stale Custom|Respawn _outactors))))) (Transformation|GetActorRotation (Utilities|Array|Get(acopy) (stale Custom|Respawn _outactors) (Math|Random|RandomIntegerinRange 0 (Utilities|Array|LastIndex (stale Custom|Respawn _outactors))))) false 0))

(event EventBeginPlay)

(event Collision|EventActorBeginOverlap
  (params (OtherActor :type Actor%20Object%20Reference)))

(event EventTick
  (params (DeltaSeconds :type Float%20%28single-precision%29)))

(fn ConstructionScript)