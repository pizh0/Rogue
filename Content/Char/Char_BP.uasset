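; Player character for a shooter, handling movement, an automatic weapon, health, ammo pickups and the HUD widget.
; Held fire loops on a short delay, spawning bullets with recoil that changes after ten shots; reload draws from reserve ammo.
; Movement adds sprint, a directional double jump and an Alt launch, alongside Ctrl slow motion and self-damage keys.
; Death disables input; Tab starts an endless loop calling Bruh on the Respawn actor.
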(event Custom|PickUpAmmo
  (params (GetAmmo :type Integer) (GetHeal :type Float%20%28single-precision%29))
  (Variables|Default|SetAmmoInv (Math|Integer|Clamp(Integer) (+ GetAmmo (Variables|Default|GetAmmoInv)) 0 (Variables|Default|GetMaxAmmoInv)))
  (Variables|Default|SetHP (Math|Float|Clamp(Float) (+ GetHeal (Variables|Default|GetHP)) 0.0 (Variables|Default|GetMaxHP))))

(event EventBeginPlay
  (Variables|Default|SetHP (Variables|Default|GetMaxHP))
  (Audio|Components|Audio|Stop (Variables|Default|GetAudio))
  (Variables|Default|SetAmmo (Variables|Default|GetMaxAmmo))
  (Variables|Default|SetAmmoInv (Variables|Default|GetDefaultAmmoInv))
  (bind _returnvalue (UserInterface|CreateWidget "/Game/UI/Char_UI.Char_UI_C" (Class|GameplayStatics|GetPlayerControllerfromID)))
  (bind _output_get (Variables|Default|SetUI_Ref _returnvalue))
  (UserInterface|Viewport|AddtoViewport _output_get 0))

(event Collision|EventActorBeginOverlap
  (params (OtherActor :type Actor%20Object%20Reference)))

(event Game|Damage|EventAnyDamage
  (params (Damage :type Float%20%28single-precision%29) (DamageType :type Damage%20Type%20Object%20Reference) (InstigatedBy :type Controller%20Object%20Reference) (DamageCauser :type Actor%20Object%20Reference))
  (bind _capsulecomponent (Variables|Collision|GetCapsuleComponent))
  (bind _returnvalue (Transformation|GetWorldLocation _capsulecomponent))
  (if (not (Variables|Default|GetDed))
    (if (<= (- (Variables|Default|GetHP) Damage) 0.0)
      (Variables|Default|SetHP (- (Variables|Default|GetHP) Damage))
      (Variables|Default|SetDed true)
      (Audio|PlaySoundatLocation "/Game/Sounds/Char/death.death" _returnvalue "0, 0, 0" 1.0 1.0 0.0 0 0 0)
      (Input|DisableInput 0)
      (Utilities|FlowControl|Delay 0.2)
      (bind _returnvalue_2 (Game|AddComponentbyClass "/Script/Engine.StaticMeshComponent" false))
      (Components|StaticMesh|SetStaticMesh _returnvalue_2 "/Game/StarterContent/Props/MaterialSphere.MaterialSphere")
      (Rendering|Material|SetMaterial _returnvalue_2 0 "/Game/Char/Nikolay.Nikolay")
      (Variables|/Script/Engine.SpringArmComponent|SetTargetArmLength (Variables|Default|GetSpringArm) 4e+02)
      (Components|DestroyComponent (Variables|Default|GetWeapon))
      (else
        (Variables|Default|SetHP (- (Variables|Default|GetHP) Damage))
        (Audio|PlaySoundatLocation "/Game/Sounds/Char/Hit_Cue.Hit_Cue" _returnvalue "0, 0, 0" 1.0 1.0 0.0 0 0 0)))))

(event EventTick
  (params (DeltaSeconds :type Float%20%28single-precision%29)))

(event EventOnLanded
  (params (Hit :type Hit%20Result%20Structure%20%28by%20ref%29))
  (bind _camera (Variables|Default|GetCamera))
  (bind _returnvalue (Transformation|GetWorldLocation _camera))
  (Variables|Default|SetDoubleJump true)
  (Audio|Components|Audio|Stop (Variables|Default|GetAudio))
  (if (>= -5e+02 (.z (Transformation|GetVelocity)))
    (Audio|PlaySoundatLocation "/Game/Sounds/Char/fallbig.fallbig" _returnvalue "0, 0, 0" 1.0 1.0 0.0 0 0 0)
    (else
      (Audio|PlaySoundatLocation "/Game/Sounds/Char/fallsmall.fallsmall" _returnvalue "0, 0, 0" 0.5 1.0 0.0 0 0 0))))

(event Input|ActionEvents|InputActionJump
  (params (Key :type Key%20Structure :default "None"))
  (bind _camera (Variables|Default|GetCamera))
  (bind _inputvector (Variables|Default|GetInputVector))
  (bind _charactermovement (Variables|Character|GetCharacterMovement))
  (bind _returnvalue (Math|Vector|GetForwardVector _camera))
  (bind _returnvalue_2 (Math|Rotator|MakeRotfromXY _inputvector _inputvector))
  (bind _returnvalue_3 (Math|Vector|RotateVector _returnvalue (Math|Rotator|MakeRotator 0.0 0.0 (.yaw _returnvalue_2))))
  (bind _returnvalue_4 (* _returnvalue_3 1e+02))
  (:Pressed
    (if (AI|Components|NavMovement|IsFalling (Variables|Character|GetCharacterMovement))
      (if (Variables|Default|GetDoubleJump)
        (Variables|/Script/Engine.MovementComponent|SetVelocity _charactermovement (/ (Variables|/Script/Engine.MovementComponent|GetVelocity _charactermovement) 2.0))
        (Character|LaunchCharacter (Math|Vector|MakeVector (.x _returnvalue_4) (.y _returnvalue_4) 7e+02) false false)
        (Variables|Default|SetDoubleJump false)
        (else
          (Development|PrintString "Bruh")))
      (else
        (Character|Jump)))))

(event Input|ActionEvents|InputActionRun
  (params (Key :type Key%20Structure :default "None"))
  (bind _charactermovement (Variables|Character|GetCharacterMovement))
  (:Pressed
    (Variables|/Script/Engine.CharacterMovementComponent|SetMaxWalkSpeed _charactermovement 1.2e+03))
  (:Released
    (Variables|/Script/Engine.CharacterMovementComponent|SetMaxWalkSpeed _charactermovement 6e+02)))

(event Input|ActionEvents|InputActionFire
  (params (Key :type Key%20Structure :default "None"))
  (bind _self self)
  (bind _boom (Variables|Default|GetBoom))
  (bind _returnvalue (Transformation|GetWorldTransform _boom))
  (:Pressed
    (bind _output_get (Variables|Default|SetFire true))
    (if _output_get :!label _label
      (if (> (Variables|Default|GetAmmo) 0)
        (bind _returnvalue_2 (Game|SpawnActorfromClass "/Game/Weapon/Common/Bullet.Bullet_C" (Math|Transform|MakeTransform (.location _returnvalue) (.rotation _returnvalue) "1,1,1") "Undefined" _self _self))
        (if (AI|Components|NavMovement|IsFalling (Variables|Character|GetCharacterMovement))
          (Default|Boomnah _returnvalue_2))
        (Components|Animation|PlayAnimation (Variables|Default|GetWeapon) "/Game/Weapon/Rifle/Anim/ShootMontage.ShootMontage" false)
        (Audio|PlaySound2D "/Game/Sounds/Char/pew-pew-lame-sound-effect.pew-pew-lame-sound-effect" 1.0 1.0 0.0 0 0)
        (bind _output_get_2 (Variables|Default|SetNOFFire (+ (Variables|Default|GetNOFFire) 1)))
        (Utilities|Recoil 0.2 _output_get_2)
        (Variables|Default|SetAmmo (- (Variables|Default|GetAmmo) 1))
        (Utilities|FlowControl|Delay 0.1)
        (goto _label)
        (else
          (Audio|PlaySound2D "/Game/Sounds/Char/anime-moan-meme.anime-moan-meme" 1.0 1.0 0.0 0 0)))))
  (:Released
    (Variables|Default|SetFire false)
    (Variables|Default|SetNOFFire 0)))

(event Input|ActionEvents|InputActionReload
  (params (Key :type Key%20Structure :default "None"))
  (bind _maxammo (Variables|Default|GetMaxAmmo))
  (:Pressed
    (if (not (== _maxammo (Variables|Default|GetAmmo)))
      (if (>= (Variables|Default|GetAmmoInv) (- _maxammo (Variables|Default|GetAmmo)))
        (Variables|Default|SetAmmoInv (- (Variables|Default|GetAmmoInv) (- _maxammo (Variables|Default|GetAmmo))))
        (Variables|Default|SetAmmo (Variables|Default|GetMaxAmmo))
        (elif (> (Variables|Default|GetAmmoInv) 0)
          (Variables|Default|SetAmmo (Variables|Default|GetAmmoInv))
          (Variables|Default|SetAmmoInv 0)
          (else
            (Audio|PlaySound2D "/Game/Sounds/Char/fallbig.fallbig" 1.0 1.0 0.0 0 0))))
      (else
        (Audio|PlaySound2D "/Game/Sounds/Char/anime-moan-meme.anime-moan-meme" 1.0 1.0 0.0 0 0)))))

(event Input|AxisEvents|InputAxisTurnUp
  (params (AxisValue :type Float%20%28single-precision%29))
  (Pawn|Input|AddControllerYawInput AxisValue))

(event Input|AxisEvents|InputAxisTurnRight
  (params (AxisValue :type Float%20%28single-precision%29))
  (Pawn|Input|AddControllerPitchInput AxisValue))

(event Input|AxisEvents|InputAxisMoveRight
  (params (AxisValue :type Float%20%28single-precision%29))
  (Pawn|Input|AddMovementInput (Math|Vector|GetRightVector (Variables|Default|GetCamera)) AxisValue false)
  (Variables|Default|SetInputVector (Math|Vector|MakeVector (stale Input|AxisEvents|InputAxisMoveFrorward AxisValue) AxisValue 0.0)))

(event Input|AxisEvents|InputAxisMoveFrorward
  (params (AxisValue :type Float%20%28single-precision%29))
  (Pawn|Input|AddMovementInput (Math|Vector|GetForwardVector (Variables|Default|GetCamera)) AxisValue false)
  (Variables|Default|SetInputVector (Math|Vector|MakeVector AxisValue (stale Input|AxisEvents|InputAxisMoveRight AxisValue) 0.0)))

(event Input|KeyboardEvents|Tab
  (params (Key :type Key%20Structure :default "None"))
  (:Pressed
    (Variables|Default|SetTabTabTab true)
    (if true :!label _label
      (bind _returnvalue (Actor|GetActorOfClass "/Game/Blueprints/Respawn.Respawn_C"))
      (bind _asrespawn (Utilities|Casting|CastToRespawn _returnvalue))
      (Default|Bruh _asrespawn)
      (Utilities|FlowControl|Delay 0.002)
      (goto _label)))
  (:Released
    (Variables|Default|SetTabTabTab true)))

(event Input|KeyboardEvents|LeftCtrl
  (params (Key :type Key%20Structure :default "None"))
  (:Pressed
    (Utilities|Time|SetGlobalTimeDilation 0.3))
  (:Released
    (Utilities|Time|SetGlobalTimeDilation 1.0)))

(event Input|KeyboardEvents|LeftAlt
  (params (Key :type Key%20Structure :default "None"))
  (bind _audio (Variables|Default|GetAudio))
  (bind _camera (Variables|Default|GetCamera))
  (bind _returnvalue (Math|Vector|GetForwardVector _camera))
  (:Pressed
    (Character|LaunchCharacter (Math|Vector|RotateVector "1000.000000, 0, 0" (Math|Rotator|MakeRotationfromAxes _returnvalue _returnvalue _returnvalue)) false false)
    (Audio|PlaySoundatLocation "/Game/Sounds/Char/launch1.launch1" (Transformation|GetWorldLocation (Variables|Default|GetCamera)) "0, 0, 0" 1.0 1.0 0.0 0 0 0)
    (if (not (Audio|Components|Audio|IsPlaying _audio)) :!label _label
      (Audio|Components|Audio|Play _audio 0.0)
      (goto _label))))

(event Input|KeyboardEvents|RightCtrl
  (params (Key :type Key%20Structure :default "None"))
  (:Pressed
    (Game|Damage|ApplyDamage self 2e+02 0 0)))

(fn ConstructionScript)